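; Base enemy AI character that patrols, shows aggro, attacks and dies into a ragdoll.
; It supplies spline patrol points in ping-pong order and exposes walk speed to behavior tree tasks.
; Attack plays a kick montage and signals when it ends, while aggro swaps the mesh to a red material.
; Point damage reduces Health, and the death check, which subtracts Damage again, triggers physics with a radial impulse from the hit.
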(event `self.ReceiveBeginPlay`
  (set `self.OriginalMaterial` (`PrimitiveComponent.GetMaterial` (`self.Mesh`) 0)))

(event `Attack`
  (`KismetSystemLibrary.PrintString` "Attacking player")
  (`|PlayMontage` (`self.Mesh`) "/Game/CloseCombatAnimSet/Animations/InPlace/Attacks/NinjaWheelKick_Montage.NinjaWheelKick_Montage"
    (:`OnCompleted`
      _)
    (:`OnInterrupted`
      _))
  (`self.AttackFinished`))

(event `GetAggro`
  (`PrimitiveComponent.SetMaterial` (`self.Mesh`) 0 "/AnimationSharing/AnimSharingRed.AnimSharingRed")
  (set `self.Aggroed` true))

(event `LoseAggro`
  (`PrimitiveComponent.SetMaterial` (`self.Mesh`) 0 (`self.OriginalMaterial`))
  (set `self.Aggroed` false))

(event `SetWalkSpeed`
  (params (`New Speed` :type "Float (double-precision)"))
  (set `CharacterMovementComponent.MaxWalkSpeed` `New Speed` (`self.CharacterMovement`)))

(event `self.ReceivePointDamage`
  (params (Damage :type "Float (single-precision)") (DamageType :type "DamageType Object Reference") (HitLocation :type "Vector Structure") (HitNormal :type "Vector Structure") (HitComponent :type "PrimitiveComponent Object Reference") (BoneName :type Name) (ShotFromDirection :type "Vector Structure") (InstigatedBy :type "Controller Object Reference") (DamageCauser :type "Actor Object Reference") (HitInfo :type "HitResult Structure (by ref)"))
  (bind _returnvalue (- (`self.Health`) Damage))
  (set `self.Health` _returnvalue)
  (if (<= _returnvalue 0.0)
    (`self.Ragdoll` HitLocation)))

(event `Ragdoll`
  (params (Origin :type "Vector Structure"))
  (bind _mesh (`self.Mesh`))
  (`PrimitiveComponent.SetSimulatePhysics` _mesh true)
  (`PrimitiveComponent.SetCollisionEnabled` _mesh "QueryAndPhysics")
  (`PrimitiveComponent.AddRadialForce` (`self.Mesh`) Origin 500.0 5000.0 "RIF_Constant" true)
  (`CharacterMovementComponent.DisableMovement` (`self.CharacterMovement`)))

(fn `GetNextPatrolPointLocation`
  (returns (Location :type "Vector Structure"))
  (`/Engine/EditorBlueprintResources/StandardMacros.IsValid` (`self.PatrolRoute`)
    (:`Is Valid`
      (set `self.Patrol Point Index` (+ (`self.Patrol Point Index`) (`self.PatrolRouteDirection`)))
      (if (or (>= (`self.Patrol Point Index`) (- (`SplineComponent.GetNumberOfSplinePoints` (`/Game/AI_Blueprints/BP_PatrolRoute.Spline` (`self.PatrolRoute`))) 1)) (<= (`self.Patrol Point Index`) 0))
        (set `self.PatrolRouteDirection` (* (`self.PatrolRouteDirection`) -1)))
      (return (`SplineComponent.GetLocationAtSplinePoint` (`/Game/AI_Blueprints/BP_PatrolRoute.Spline` (`self.PatrolRoute`)) (`self.Patrol Point Index`) "World")))
    (:`Is Not Valid`
      (`KismetSystemLibrary.PrintString` "No patrol route found")
      (return (0.0 0.0 0.0)))))

(fn `UserConstructionScript`)