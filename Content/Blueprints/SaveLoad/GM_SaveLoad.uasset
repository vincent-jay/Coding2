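; GM_SaveLoad is a game mode that persists player stats through an SG_PlayerStats save object in the PlayerSave slot.
; On BeginPlay it loads an existing save and copies Stamina onto the BP_ThirdPersonCharacter, or creates a fresh save object if none exists.
; SavePlayerStats writes the held object as it stands, without reading the character, and prints the result.
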(event `self.ReceiveBeginPlay`
  (`KismetSystemLibrary.PrintString` "Loading the SaveLoad Game Mode" true true (struct :`R` 0.47881 :`G` 0.099822 :`B` 1.0 :`A` 1.0) 10.0)
  (`self.Load Player Stats`))

(event `Load Player Stats`
  (bind _returnvalue (`GameplayStatics.DoesSaveGameExist` "PlayerSave"))
  (if _returnvalue
    (bind _returnvalue_2 (`GameplayStatics.LoadGameFromSlot` "PlayerSave"))
    (bind _assg_player_stats (cast `/Game/Blueprints/SaveLoad/SG_PlayerStats` _returnvalue_2))
    (set `self.SG_PlayerStats` _assg_player_stats)
    (bind _asbp_third_person_character (cast `/Game/ThirdPerson/Blueprints/BP_ThirdPersonCharacter` (`GameplayStatics.GetPlayerCharacter` 0)))
    (set `/Game/ThirdPerson/Blueprints/BP_ThirdPersonCharacter.Stamina` (`/Game/Blueprints/SaveLoad/SG_PlayerStats.Stamina` (`self.SG_PlayerStats`)) _asbp_third_person_character) ; Setting the players stamina\nto the saved stamina
    (`KismetSystemLibrary.PrintString` "PlayerStats have been loaded." true true (struct :`R` 0.47881 :`G` 0.099822 :`B` 1.0 :`A` 1.0) 10.0)
    (else
      (bind _returnvalue_3 (`GameplayStatics.CreateSaveGameObject` "/Game/Blueprints/SaveLoad/SG_PlayerStats.SG_PlayerStats_C"))
      (set `self.SG_PlayerStats` _returnvalue_3))))

(event `Save Player Stats`
  (bind _returnvalue (`GameplayStatics.SaveGameToSlot` (`self.SG_PlayerStats`) "PlayerSave"))
  (if _returnvalue
    (`KismetSystemLibrary.PrintText` "Player Stats Written to Save Game File." true true (struct :`R` 0.47881 :`G` 0.099822 :`B` 1.0 :`A` 1.0) 10.0)
    (else
      (`KismetSystemLibrary.PrintText` "Player Stats Could Not Be Written to Save Game File." true true (struct :`R` 1.0 :`G` 0.770775 :`A` 1.0) 10.0))))

(fn `UserConstructionScript`)