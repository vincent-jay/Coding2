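; BP_Door is a locked door that opens when the third-person character enters its collision volume while holding a key.
; The overlap event casts to BP_ThirdPersonCharacter, decrements its Keys count and plays the TL_OpenDoor timeline, or prints that a key is needed.
; The timeline lerps the Door component's relative Z to slide it downward and sets Opened, which blocks further triggers; nothing closes it again.
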(event `self.Collision.OnComponentBeginOverlap`
  (params (OverlappedComponent :type "PrimitiveComponent Object Reference") (OtherActor :type "Actor Object Reference") (OtherComp :type "PrimitiveComponent Object Reference") (OtherBodyIndex :type Integer) (bFromSweep :type Boolean) (SweepResult :type "HitResult Structure (by ref)"))
  (if (not (`self.Opened`))
    (bind _asbp_third_person_character (cast `/Game/ThirdPerson/Blueprints/BP_ThirdPersonCharacter` OtherActor))
    (bind _keys (`/Game/ThirdPerson/Blueprints/BP_ThirdPersonCharacter.Keys` _asbp_third_person_character))
    (if (> _keys 0)
      (`/Engine/EditorBlueprintResources/StandardMacros.DecrementInt` _keys
        (:`  `
          (`KismetSystemLibrary.PrintString` "You used a key." true true (struct :`R` 0.08581 :`G` 1.0 :`A` 1.0))
          (bind (_direction _newtrack_0) (`Timeline|TL_OpenDoor`)
            (:`Update`
              (`SceneComponent.K2_SetRelativeLocation` (`self.Door`) (`KismetMathLibrary.MakeVector` 0.0 0.0 (`KismetMathLibrary.Lerp` 137.0 -130.0 _newtrack_0)) false false)
              (set `self.Opened` true)))))
      (else
        (`KismetSystemLibrary.PrintString` "You need a key." true true (struct :`R` 1.0 :`G` 0.25684 :`A` 1.0))))))

(fn `UserConstructionScript`)