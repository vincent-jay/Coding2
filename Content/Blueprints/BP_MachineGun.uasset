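; BP_MachineGun is a weapon actor that can be picked up, used and dropped, with firing so far only a "Pew pew pew" text print.
; Pickup snaps it to the given skeletal mesh's hand_r socket and disables body collision.
; Drop detaches it, restores collision and simulates physics on the body for a brief delay.
; BeginPlay caches the body's relative location, unused here, and a root-to-body reposition node is left unwired.
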(event `self.ReceiveBeginPlay`
  (set `self.Relative Location` (`SceneComponent.RelativeLocation` (`self.MachineGunBody`))))

(event `/Game/Blueprints/BPI_Item.Pickup`
  (params (SkeletalMesh :type "SkeletalMeshComponent Object Reference"))
  (`KismetSystemLibrary.PrintText` (`|FormatText` "{name} is getting picked up and attached to {mesh}." (`KismetSystemLibrary.GetObjectName` self) SkeletalMesh) true true (struct :`R` 1.0 :`G` 0.130801 :`B` 0.899906 :`A` 1.0) 5.0)
  (`self.K2_AttachToComponent` SkeletalMesh "hand_r" "SnapToTarget" "SnapToTarget" "SnapToTarget")
  (`PrimitiveComponent.SetCollisionEnabled` (`self.MachineGunBody`) "NoCollision"))

(event `/Game/Blueprints/BPI_Item.Use Primary`
  (`KismetSystemLibrary.PrintText` "Pew pew pew" true true (struct :`R` 1.0 :`G` 0.770775 :`A` 1.0)))

(event `/Game/Blueprints/BPI_Item.Drop`
  (bind _machinegunbody (`self.MachineGunBody`))
  (`self.K2_DetachFromActor` "KeepWorld" "KeepWorld" "KeepWorld")
  (`PrimitiveComponent.SetSimulatePhysics` _machinegunbody true)
  (`PrimitiveComponent.SetCollisionEnabled` _machinegunbody "QueryAndPhysics")
  (`KismetSystemLibrary.Delay` 1.0)
  (`PrimitiveComponent.SetSimulatePhysics` _machinegunbody false))

(fn `UserConstructionScript`)