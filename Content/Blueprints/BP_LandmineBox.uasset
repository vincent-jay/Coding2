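; BP_LandmineBox is a carryable item that a player uses up to place a landmine on the ground.
; Pickup snaps it to the hand_r socket with collision off, and Drop detaches it, restores collision and simulates physics briefly before switching physics off.
; UsePrimary destroys the box, traces down from the player's capsule and spawns a BP_Landmine at the impact point, without checking for a hit.
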(event `self.Use Primary`
  (params (Player :type "/Game/ThirdPerson/Blueprints/BP_ThirdPersonCharacter Object Reference"))
  (bind _returnvalue (`SceneComponent.K2_GetComponentLocation` (`Character.CapsuleComponent` Player)))
  (`self.K2_DestroyActor`)
  (bind _outhit (`KismetSystemLibrary.LineTraceSingle` _returnvalue (- _returnvalue (0.0 0.0 500.0)) "TraceTypeQuery1" false (`|MakeArray` Player :!type "Actor Object Reference")))
  (`|SpawnActorFromClass` "/Game/Blueprints/BP_Landmine.BP_Landmine_C" (`KismetMathLibrary.MakeTransform` (`.ImpactPoint` (`GameplayStatics.BreakHitResult` _outhit))) "Undefined" "MultiplyWithRoot" null null))

(event `self.Drop`
  (bind _cube (`self.Cube`))
  (`self.K2_DetachFromActor` "KeepWorld" "KeepWorld")
  (`PrimitiveComponent.SetSimulatePhysics` _cube true)
  (`PrimitiveComponent.SetCollisionEnabled` _cube "QueryAndPhysics")
  (`KismetSystemLibrary.Delay` 1.0)
  (`PrimitiveComponent.SetSimulatePhysics` _cube false))

(event `self.Pickup`
  (params (SkeletalMesh :type "SkeletalMeshComponent Object Reference"))
  (`KismetSystemLibrary.PrintText` (`|FormatText` "{name} is getting picked up and attached to {mesh}." (`KismetSystemLibrary.GetObjectName` self) _) true true (struct :`R` 1.0 :`G` 0.130801 :`B` 0.899906 :`A` 1.0) 5.0)
  (`self.K2_AttachToComponent` SkeletalMesh "hand_r" "SnapToTarget" "SnapToTarget" "KeepRelative")
  (`PrimitiveComponent.SetCollisionEnabled` (`self.Cube`) "NoCollision"))

(fn `UserConstructionScript`)