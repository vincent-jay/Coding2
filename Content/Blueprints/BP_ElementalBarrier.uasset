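; BP_ElementalBarrier is a labelled hazard barrier that only a character with the matching elemental immunity survives.
; On BeginPlay its TextRender shows the barrier's ElementalType.
; When a BP_ThirdPersonCharacter overlaps the Cube, its ElementalImmunity is compared to that type.
; A mismatch prints a red death message and, after a short delay, quits the game outright.
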(event `self.ReceiveBeginPlay`
  (`TextRenderComponent.K2_SetText` (`self.TextRender`) (`KismetTextLibrary.Conv_StringToText` (`KismetStringLibrary.Concat_StrStr` "Barrier of " (`KismetTextLibrary.Conv_TextToString` (`|GenericToText` (`self.ElementalType`)))))))

(event `self.Cube.OnComponentBeginOverlap`
  (params (OverlappedComponent :type "PrimitiveComponent Object Reference") (OtherActor :type "Actor Object Reference") (OtherComp :type "PrimitiveComponent Object Reference") (OtherBodyIndex :type Integer) (bFromSweep :type Boolean) (SweepResult :type "HitResult Structure (by ref)"))
  (bind _asbp_third_person_character (cast `/Game/ThirdPerson/Blueprints/BP_ThirdPersonCharacter` OtherActor))
  (if (not (`|EnumEquality` (`/Game/ThirdPerson/Blueprints/BP_ThirdPersonCharacter.ElementalImmunity` _asbp_third_person_character) (`self.ElementalType`)))
    (`KismetSystemLibrary.PrintString` "YOU ARE DEAD!!" true true (struct :`R` 1.0 :`G` 0.00334 :`A` 1.0))
    (`KismetSystemLibrary.Delay` 2.0)
    (`KismetSystemLibrary.QuitGame` null "Quit")))

(fn `UserConstructionScript`)