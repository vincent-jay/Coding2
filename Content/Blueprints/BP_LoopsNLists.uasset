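; Demo Blueprint that shows looping and array iteration through on-screen debug prints, all started from BeginPlay.
; DelayLoop increments and prints a counter, waits briefly, then calls itself, forming an endless timed loop without Tick.
; PrintColors shuffles the TextColors array, prints each entry's position in that color with a for-each loop, then prints a completion message.
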(event `self.ReceiveBeginPlay`
  (`KismetSystemLibrary.PrintString` "Loops + lists is active.")
  (`self.Delay Loop`)
  (`self.Print Colors`))

(event `Delay Loop`
  (bind _result (`/Engine/EditorBlueprintResources/StandardMacros.IncrementInt` (`self.DelayLoopCount`))
    (:`  `
      (`KismetSystemLibrary.PrintString` (`KismetStringLibrary.Concat_StrStr` "Starting delay loop: #" (`KismetStringLibrary.Conv_IntToString` _result)))
      (`KismetSystemLibrary.Delay` 0.5)
      (`self.Delay Loop`))))

(event `Print Colors`
  (bind _textcolors (`self.TextColors`))
  (`KismetArrayLibrary.Array_Shuffle` _textcolors)
  (for (_array_element _array_index) _textcolors
    (`KismetSystemLibrary.PrintString` (`KismetStringLibrary.Concat_StrStr` "Color #" (`KismetStringLibrary.Conv_IntToString` (+ _array_index 1))) true true _array_element 5.0))
  (`KismetSystemLibrary.PrintString` "Done printing colors." true true (struct :`A` 1.0)))

(fn `UserConstructionScript`)