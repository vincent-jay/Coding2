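; BP_EnemySpawner populates the level with randomized AI enemies once at BeginPlay.
; It finds every BP_EnemySpawnPoint and, on a coin flip for each, spawns a BP_AiMoveTo at that point's transform.
; Each spawned AI gets a random name from PossibleNames on its AINameText, a random Quinn or Manny mesh, and randomly picked materials for both slots.
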(event `self.ReceiveBeginPlay`
  (`KismetSystemLibrary.PrintString` "Enemy spawner is active." true true (struct :`R` 1.0 :`G` 0.420618 :`A` 1.0))
  (bind _outactors (`GameplayStatics.GetAllActorsOfClass` "/Game/Blueprints/BP_EnemySpawnPoint.BP_EnemySpawnPoint_C"))
  (for _array_element _outactors
    (if (`KismetMathLibrary.RandomBool`)
      (bind _returnvalue (`|SpawnActorFromClass` "/Game/AI_Blueprints/BP_AiMoveTo.BP_AiMoveTo_C" (`self.GetTransform` _array_element) "Undefined" "MultiplyWithRoot" null null))
      (`TextRenderComponent.K2_SetText` (`/Game/AI_Blueprints/BP_AiMoveTo.AINameText` _returnvalue) (`KismetArrayLibrary.Array_Random` (`self.PossibleNames`)))
      (bind _mesh (`Character.Mesh` _returnvalue))
      (`SkeletalMeshComponent.SetSkeletalMeshAsset` _mesh (select `bool` (`KismetMathLibrary.RandomBool`) :`false` "/Game/Characters/Mannequins/Meshes/SKM_Manny_Simple.SKM_Manny_Simple" :`true` "/Game/Characters/Mannequins/Meshes/SKM_Quinn_Simple.SKM_Quinn_Simple" :!type "SkeletalMesh Object Reference"))
      (`PrimitiveComponent.SetMaterial` _mesh 0 (select `bool` (`KismetMathLibrary.RandomBool`) :`false` "/AnimationSharing/AnimSharingBlue.AnimSharingBlue" :`true` "/DatasmithContent/Materials/AliasReference.AliasReference" :!type "MaterialInterface Object Reference"))
      (`PrimitiveComponent.SetMaterial` _mesh 1 (select `bool` (`KismetMathLibrary.RandomBool`) :`false` "/Game/Characters/Mannequins/Materials/Instances/Manny/MI_Manny_01.MI_Manny_01" :`true` "/Game/Characters/Mannequins/Materials/Instances/Manny/MI_Manny_02.MI_Manny_02" :!type "MaterialInterface Object Reference")))))

(fn `UserConstructionScript`)