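; BP_Apple is a holdable apple item that adds one to the player's Health when used.
; UsePrimary increments Health, prints the new value in green and destroys the apple.
; Pickup prints a message, snaps the apple to the hand_r socket of the given skeletal mesh and disables Sphere collision.
; Drop detaches it and restores collision, simulating physics on the Sphere for one second before freezing it.
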(event `/Game/Blueprints/BPI_Item.Use Primary`
  (params (Player :type "/Game/ThirdPerson/Blueprints/BP_ThirdPersonCharacter Object Reference"))
  (bind _result (`/Engine/EditorBlueprintResources/StandardMacros.IncrementInt` (`/Game/ThirdPerson/Blueprints/BP_ThirdPersonCharacter.Health` Player))
    (:`  `
      (`KismetSystemLibrary.PrintText` (`|FormatText` "I have {health} health now." _result) true true (struct :`R` 0.021266 :`G` 1.0 :`A` 1.0))
      (`self.K2_DestroyActor`))))

(event `/Game/Blueprints/BPI_Item.Drop`
  (bind _sphere (`self.Sphere`))
  (`self.K2_DetachFromActor` "KeepWorld" "KeepWorld" "KeepWorld")
  (`PrimitiveComponent.SetSimulatePhysics` _sphere true)
  (`PrimitiveComponent.SetCollisionEnabled` _sphere "QueryAndPhysics")
  (`KismetSystemLibrary.Delay` 1.0)
  (`PrimitiveComponent.SetSimulatePhysics` _sphere false))

(event `/Game/Blueprints/BPI_Item.Pickup`
  (params (SkeletalMesh :type "SkeletalMeshComponent Object Reference"))
  (`KismetSystemLibrary.PrintText` (`|FormatText` "{name} is getting picked up and attached to {mesh}." (`KismetSystemLibrary.GetObjectName` self) _) true true (struct :`R` 1.0 :`G` 0.130801 :`B` 0.899906 :`A` 1.0) 5.0)
  (`self.K2_AttachToComponent` SkeletalMesh "hand_r" "SnapToTarget" "SnapToTarget" "SnapToTarget")
  (`PrimitiveComponent.SetCollisionEnabled` (`self.Sphere`) "NoCollision"))

(fn `UserConstructionScript`)