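; BP_ManaPickup is a carryable, single-use item that raises one player stat, presumably mana, by 0.25.
; Pickup attaches it to the skeletal mesh's hand_r socket and turns off Sphere collision.
; Drop detaches it, restores collision and simulates physics on the Sphere for one second before switching physics off.
; UsePrimary applies the stat change through the player's ChangeStat, then destroys the actor.
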(event `self.Use Primary`
  (params (Player :type "/Game/ThirdPerson/Blueprints/BP_ThirdPersonCharacter Object Reference"))
  (`/Game/ThirdPerson/Blueprints/BP_ThirdPersonCharacter.Change Stat` Player "NewEnumerator1" 0.25)
  (`self.K2_DestroyActor`))

(event `self.Drop`
  (bind _sphere (`self.Sphere`))
  (`self.K2_DetachFromActor` "KeepWorld" "KeepWorld")
  (`PrimitiveComponent.SetSimulatePhysics` _sphere true)
  (`PrimitiveComponent.SetCollisionEnabled` _sphere "QueryAndPhysics")
  (`KismetSystemLibrary.Delay` 1.0)
  (`PrimitiveComponent.SetSimulatePhysics` _sphere false))

(event `self.Pickup`
  (params (SkeletalMesh :type "SkeletalMeshComponent Object Reference"))
  (`KismetSystemLibrary.PrintText` (`|FormatText` "{name} is getting picked up and attached to {mesh}." (`KismetSystemLibrary.GetObjectName` self) _) true true (struct :`R` 1.0 :`G` 0.130801 :`B` 0.899906 :`A` 1.0) 5.0)
  (`self.K2_AttachToComponent` SkeletalMesh "hand_r" "SnapToTarget" "SnapToTarget" "KeepRelative")
  (`PrimitiveComponent.SetCollisionEnabled` (`self.Sphere`) "NoCollision"))

(fn `UserConstructionScript`)